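; Game instance for Astral Defence that owns the player's gameplay, input, audio and video settings across the session.
; On Init it loads each category from its own SaveGame slot, creating and saving a fresh object when loading fails, then applies them; Shutdown saves all four.
; Video and audio values are pushed to GameUserSettings, while the gameplay and input apply functions are empty stubs.
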(event EventInit
  (CallFunction|LoadAllSettings)
  (CallFunction|ApplyAllSettings))

(event EventShutdown
  (CallFunction|SaveAllSettings))

(fn SaveGameplaySettings
  (bind _returnvalue (SaveGame|SaveGametoSlot (Variables|Default|GetGameplaySettings) (Variables|Default|GetGameplaySettingsSlot)))
  (if _returnvalue
    (Development|PrintString "Successfully saved Gameplay Settings")
    (else
      (Development|PrintString "Failed to save Gameplay Settings"))))

(fn SaveInputSettings
  (bind _returnvalue (SaveGame|SaveGametoSlot (Variables|Default|GetInputSettings) (Variables|Default|GetInputSettingsSlot)))
  (if _returnvalue
    (Development|PrintString "Successfully save Input Settings")
    (else
      (Development|PrintString "Failed to save Input Settings"))))

(fn SaveAudioSettings
  (bind _returnvalue (SaveGame|SaveGametoSlot (Variables|Default|GetAudioSettings) (Variables|Default|GetAudioSettingsSlot)))
  (if _returnvalue
    (Development|PrintString "Successfully saved Audio Settings")
    (else
      (Development|PrintString "Failed to save Audio Settings"))))

(fn SaveVideoSettings
  (bind _returnvalue (SaveGame|SaveGametoSlot (Variables|Default|GetVideoSettings) (Variables|Default|GetVideoSettingsSlot)))
  (if _returnvalue
    (Development|PrintString "Successfully saved Video Settings")
    (else
      (Development|PrintString "Failed to save Video Settings"))))

(fn LoadGameplaySettings
  (bind _gameplaysettingsslot (Variables|Default|GetGameplaySettingsSlot))
  (bind _returnvalue (SaveGame|LoadGamefromSlot _gameplaysettingsslot))
  (bind _asgameplay_settings (Utilities|Casting|CastToGameplaySettings _returnvalue)
    (:then
      (Variables|Default|SetGameplaySettings _asgameplay_settings)
      (Development|PrintString "Successfully loaded Gameplay Settings"))
    (:CastFailed
      (Development|PrintString "Failed to load Gameplay Settings")
      (bind _returnvalue_2 (SaveGame|CreateSaveGameObject "/Game/Settings/GameplaySettings.GameplaySettings_C"))
      (bind _output_get (Variables|Default|SetGameplaySettings _returnvalue_2))
      (bind _returnvalue_3 (SaveGame|SaveGametoSlot _output_get _gameplaysettingsslot))
      (if _returnvalue_3
        (Development|PrintString "Successfully created initial Gameplay Settings")
        (else
          (Development|PrintString "Failed to create initial Gameplay Settings"))))))

(fn LoadInputSettings
  (bind _inputsettingsslot (Variables|Default|GetInputSettingsSlot))
  (bind _returnvalue (SaveGame|LoadGamefromSlot _inputsettingsslot))
  (bind _asinput_settings (Utilities|Casting|CastToInputSettings _returnvalue)
    (:then
      (Variables|Default|SetInputSettings _asinput_settings)
      (Development|PrintString "Successfully loaded Input Settings"))
    (:CastFailed
      (Development|PrintString "Failed to load Input Settings")
      (bind _returnvalue_2 (SaveGame|CreateSaveGameObject "/Game/Settings/InputSettings.InputSettings_C"))
      (bind _output_get (Variables|Default|SetInputSettings _returnvalue_2))
      (bind _returnvalue_3 (SaveGame|SaveGametoSlot _output_get _inputsettingsslot))
      (if _returnvalue_3
        (Development|PrintString "Successfully created initial Input Settings")
        (else
          (Development|PrintString "Failed to create initial Input Settings"))))))

(fn LoadAudioSettings
  (bind _audiosettingsslot (Variables|Default|GetAudioSettingsSlot))
  (bind _returnvalue (SaveGame|LoadGamefromSlot _audiosettingsslot))
  (bind _asaudio_settings (Utilities|Casting|CastToAudioSettings _returnvalue)
    (:then
      (Variables|Default|SetAudioSettings _asaudio_settings)
      (Development|PrintString "Successfully loaded Audio Settings"))
    (:CastFailed
      (Development|PrintString "Failed to load Audio Settings")
      (bind _returnvalue_2 (SaveGame|CreateSaveGameObject "/Game/Settings/AudioSettings.AudioSettings_C"))
      (bind _output_get (Variables|Default|SetAudioSettings _returnvalue_2))
      (bind _returnvalue_3 (SaveGame|SaveGametoSlot _output_get _audiosettingsslot))
      (if _returnvalue_3
        (Development|PrintString "Successfully created initial Audio Settings")
        (else
          (Development|PrintString "Failed to create initial Audio Settings"))))))

(fn LoadVideoSettings
  (bind _videosettingsslot (Variables|Default|GetVideoSettingsSlot))
  (bind _returnvalue (SaveGame|LoadGamefromSlot _videosettingsslot))
  (bind _asvideo_settings (Utilities|Casting|CastToVideoSettings _returnvalue)
    (:then
      (Variables|Default|SetVideoSettings _asvideo_settings)
      (Development|PrintString "Successfully loaded Video Settings"))
    (:CastFailed
      (Development|PrintString "Failed to load Video Settings")
      (bind _returnvalue_2 (SaveGame|CreateSaveGameObject "/Game/Settings/VideoSettings.VideoSettings_C"))
      (bind _output_get (Variables|Default|SetVideoSettings _returnvalue_2))
      (bind _returnvalue_3 (SaveGame|SaveGametoSlot _output_get _videosettingsslot))
      (if _returnvalue_3
        (Development|PrintString "Successfully created initial Video Settings")
        (else
          (Development|PrintString "Failed to create initial Video Settings"))))))

(fn LoadAllSettings
  (Utilities|FlowControl|Sequence
    (:then_0
      (CallFunction|LoadInputSettings))
    (:then_1
      (CallFunction|LoadGameplaySettings))
    (:then_2
      (CallFunction|LoadAudioSettings))
    (:then_3
      (CallFunction|LoadVideoSettings))))

(fn SaveAllSettings
  (Utilities|FlowControl|Sequence
    (:then_0
      (CallFunction|SaveInputSettings))
    (:then_1
      (CallFunction|SaveGameplaySettings))
    (:then_2
      (CallFunction|SaveAudioSettings))
    (:then_3
      (CallFunction|SaveVideoSettings))))

(fn ApplyAllSettings
  (Utilities|FlowControl|Sequence
    (:then_0
      (CallFunction|ApplyInputSettings))
    (:then_1
      (CallFunction|ApplyGameplaySettings))
    (:then_2
      (CallFunction|ApplyAudioSettings))
    (:then_3
      (CallFunction|ApplyVideoSettings))))

(fn ApplyVideoSettings
  (bind _videosettings (Variables|Default|GetVideoSettings))
  (bind _returnvalue (Settings|GetGameUserSettings))
  (Utilities|FlowControl|Sequence
    (:then_0
      (Class|GameUserSettings|SetVisualEffectQuality _returnvalue (Variables|/Game/Settings/VideoSettings.VideoSettings_C|GetVisualEffectQuality _videosettings)))
    (:then_1
      (Class|GameUserSettings|SetViewDistanceQuality _returnvalue (Variables|/Game/Settings/VideoSettings.VideoSettings_C|GetViewDistanceQuality _videosettings)))
    (:then_2
      (Class|GameUserSettings|SetTextureQuality _returnvalue (Variables|/Game/Settings/VideoSettings.VideoSettings_C|GetTextureQuality _videosettings)))
    (:then_3
      (Class|GameUserSettings|SetShadowQuality _returnvalue (Variables|/Game/Settings/VideoSettings.VideoSettings_C|GetShadowQuality _videosettings)))
    (:then_4
      (Class|GameUserSettings|SetPostProcessingQuality _returnvalue (Variables|/Game/Settings/VideoSettings.VideoSettings_C|GetPostProcessingQuality _videosettings)))
    (:then_5
      (Class|GameUserSettings|SetFoliageQuality _returnvalue (Variables|/Game/Settings/VideoSettings.VideoSettings_C|GetFoliageQuality _videosettings)))
    (:then_6
      (Class|GameUserSettings|SetAntiAliasingQuality _returnvalue (Variables|/Game/Settings/VideoSettings.VideoSettings_C|GetAntiAliasingQuality _videosettings)))
    (:then_7
      (Class|GameUserSettings|SetFrameRateLimit _returnvalue (Variables|/Game/Settings/VideoSettings.VideoSettings_C|GetFrameRateLimit _videosettings)))
    (:then_11
      (Class|GameUserSettings|ApplySettings _returnvalue false))))

(fn ApplyAudioSettings
  (bind _returnvalue (Settings|GetGameUserSettings))
  (Class|GameUserSettings|SetAudioQualityLevel _returnvalue (Variables|/Game/Settings/AudioSettings.AudioSettings_C|GetAudioQuality (Variables|Default|GetAudioSettings)))
  (Class|GameUserSettings|ApplySettings _returnvalue false))

(fn ApplyGameplaySettings)

(fn ApplyInputSettings)