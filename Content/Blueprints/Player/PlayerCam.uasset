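; Player camera actor that flies over the level with a spring-arm camera, controlled by mouse and movement axes.
; MoveForward and MoveRight offset the actor locally without sweep, and the mouse wheel changes spring-arm length to zoom, with no clamp.
; Holding the right mouse button hides the cursor and opens two gates that let mouse X yaw the actor and mouse Y pitch the spring arm.
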(event EventBeginPlay
  (Variables|/Script/Engine.PlayerController|SetbShowMouseCursor (Game|GetPlayerController 0) true))

(event Input|AxisEvents|InputAxisMoveForward
  (params (AxisValue :type Float%20%28single-precision%29))
  (Transformation|AddActorLocalOffset (Math|Vector|MakeVector (* AxisValue (Variables|Default|GetSpeed)) 0.0 0.0) false false))

(event Input|AxisEvents|InputAxisMoveRight
  (params (AxisValue :type Float%20%28single-precision%29))
  (Transformation|AddActorLocalOffset (Math|Vector|MakeVector 0.0 (* AxisValue (Variables|Default|GetSpeed)) 0.0) false false))

(event Input|MouseEvents|MouseX
  (params (AxisValue :type Float%20%28single-precision%29))
  (Utilities|FlowControl|Gate true
    (:Exit
      (Class|Actor|AddActorWorldRotation (Math|Rotator|MakeRotator 0.0 0.0 (* AxisValue (Variables|Default|GetRotateSpeed)))))))

(event Input|MouseEvents|MouseY
  (params (AxisValue :type Float%20%28single-precision%29))
  (Utilities|FlowControl|Gate true
    (:Exit
      (Transformation|AddLocalRotation (Variables|Default|GetSpringArm) (Math|Rotator|MakeRotator 0.0 (* AxisValue (Variables|Default|GetRotateSpeed)) 0.0) false false))))

(event Input|MouseEvents|MouseWheelUp
  (params (Key :type Key%20Structure))
  (bind _springarm (Variables|Default|GetSpringArm))
  (:Pressed
    (Variables|/Script/Engine.SpringArmComponent|SetTargetArmLength _springarm (- (Variables|/Script/Engine.SpringArmComponent|GetTargetArmLength _springarm) 6e+01))))

(event Input|MouseEvents|MouseWheelDown
  (params (Key :type Key%20Structure))
  (bind _springarm (Variables|Default|GetSpringArm))
  (:Pressed
    (Variables|/Script/Engine.SpringArmComponent|SetTargetArmLength _springarm (+ (Variables|/Script/Engine.SpringArmComponent|GetTargetArmLength _springarm) 6e+01))))

(event Input|MouseEvents|RightMouseButton
  (params (Key :type Key%20Structure))
  (bind _returnvalue (Game|GetPlayerController 0))
  (:Pressed
    (Variables|/Script/Engine.PlayerController|SetbShowMouseCursor _returnvalue false)
    (Utilities|FlowControl|Sequence
      (:then_0
        (Utilities|FlowControl|Gate true) ; enters at Open
      )
      (:then_1
        (Utilities|FlowControl|Gate true) ; enters at Open
      )))
  (:Released
    (Variables|/Script/Engine.PlayerController|SetbShowMouseCursor _returnvalue true)
    (Utilities|FlowControl|Sequence
      (:then_0
        (Utilities|FlowControl|Gate true) ; enters at Close
      )
      (:then_1
        (Utilities|FlowControl|Gate true) ; enters at Close
      ))))

(fn ConstructionScript)