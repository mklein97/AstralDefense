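; BP_EnemyAI is an enemy that marches to a fixed world location and damages every BP_PlayerBase when it arrives, destroying itself.
; Tick starts the AI move while not already moving and turns the health bar to face the player camera.
; Projectile-tagged overlaps on the Wiggler component reduce clamped health, and death awards money to every BP_PlayerBase.
; BeginPlay passes the enemy to its EnemyHealth widget.
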(event OnComponentBeginOverlap(wiggler)
  (params (OverlappedComponent :type Primitive%20Component%20Object%20Reference) (OtherActor :type Actor%20Object%20Reference) (OtherComp :type Primitive%20Component%20Object%20Reference) (OtherBodyIndex :type Integer) (bFromSweep :type Boolean) (SweepResult :type Hit%20Result%20Structure%20%28by%20ref%29))
  (if (Actor|ActorHasTag OtherActor "Projectile")
    (Actor|DestroyActor OtherActor)
    (CallFunction|TakeDamage self 2e+01)
    (if (<= (Variables|Default|GetAiHealth) 0.0)
      (Actor|DestroyActor self)
      (bind _outactors (Actor|GetAllActorsOfClass "/Game/Blueprints/Base/BP_PlayerBase.BP_PlayerBase_C"))
      (for _array_element _outactors
        (bind _asbp_player_base (Utilities|Casting|CastToBP_PlayerBase _array_element))
        (bind _output_get (Variables|/Script/TowerDefense.PlayerBase|SetMoney _asbp_player_base (+ (Variables|/Script/TowerDefense.PlayerBase|GetMoney _asbp_player_base) 100)))
        (Development|PrintString (Utilities|String|ToString(Integer) _output_get))))))

(event Custom|Tick%202
  (params (deltaSeconds :type Float%20%28single-precision%29))
  (if (not (Variables|Default|GetisMoving))
    (AI|AIMoveTo self "70.000000,-4180.000000,146.000000" 0 1.0 false
      (:then
        (Variables|Default|SetisMoving true))
      (:OnSuccess
        (Actor|DestroyActor self)
        (bind _outactors (Actor|GetAllActorsOfClass "/Game/Blueprints/Base/BP_PlayerBase.BP_PlayerBase_C"))
        (for _array_element _outactors
          (bind _asbp_player_base (Utilities|Casting|CastToBP_PlayerBase _array_element))
          (Variables|/Script/TowerDefense.PlayerBase|SetHealth _asbp_player_base (- (Variables|/Script/TowerDefense.PlayerBase|GetHealth _asbp_player_base) 5)))))))

(event Custom|Tick%201
  (params (deltaSeconds :type Float%20%28single-precision%29))
  (CallFunction|RotateHealthbartoPlayer))

(event EventTick
  (params (DeltaSeconds :type Float%20%28single-precision%29))
  (CallFunction|Tick2 0.0)
  (CallFunction|Tick1 0.0))

(event EventBeginPlay
  (EditorScripting|ActorEditing|SetActorLabel "Enemy" false)
  (bind _asenemy_health (Utilities|Casting|CastToEnemyHealth (UserInterface|GetUserWidgetObject (Variables|Default|Gethealthbar))))
  (Variables|/Game/Blueprints/Enemies/EnemyHealth.EnemyHealth_C|SetEnemy _asenemy_health self))

(fn ConstructionScript)

(fn RotateHealthbartoPlayer
  (bind _healthbar (Variables|Default|Gethealthbar))
  (Transformation|SetWorldRotation _healthbar (Math|Rotator|FindLookatRotation (Transformation|GetWorldLocation _healthbar) (Camera|GetCameraLocation (Game|GetPlayerCameraManager 0))) false false))

(fn TakeDamage
  (params (Damage :type Float%20%28single-precision%29))
  (bind _output_get (Variables|Default|SetAiHealth (Math|Float|Clamp(Float) (- (Variables|Default|GetAiHealth) Damage) 0.0 1e+02)))
  (Variables|Default|SetAiHealthPercent (/ _output_get 1e+02)))